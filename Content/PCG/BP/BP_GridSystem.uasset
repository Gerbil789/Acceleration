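; BP_GridSystem is a procedural hex-grid generator that builds a map of forest, field and rock tiles in the construction script.
; It spawns child actors over Width and Height, spacing them from the tile mesh's bounds and an Offset multiplier, with a FlipFlop staggering alternate rows.
; Weighted random picks choose forest by ForestDensity, otherwise mostly rock with some field.
; BeginPlay gathers forest tiles but does nothing with them.
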(event EventBeginPlay
  (bind _filteredarray (Utilities|Array|FilterArray (Actor|GetAllChildActors true) "/Game/Blueprints/BP_ForestTile.BP_ForestTile_C"))
  (for _array_element _filteredarray
    _))

(fn ConstructionScript
  (Variables|Default|SetTileRadius (.x (.max (StaticMesh|GetBoundingBox (Variables|Default|GetTileMesh)))))
  ;[1 1 1] Height loop
  (for _index (range 0 (- (Variables|Default|GetHeight) 1))
    ;[1 1 1] Width loop
    (for _index_2 (range 0 (- (Variables|Default|GetWidth) 1))
      (bind _returnvalue (AddComponent|AddChildActorComponent false (Math|Transform|MakeTransform (Math|Vector|MakeVector (+ (* _index_2 (* (Variables|Default|GetTileRadius) (Variables|Default|GetOffset))) (Variables|Default|GetRowOffset)) (* _index (* (* (/ (Variables|Default|GetTileRadius) 2.0) (Math|Float|Sqrt 3.0)) (Variables|Default|GetOffset))) 0.0) "0, 0, 0" "1.000000,1.000000,1.000000")))
      (if (Math|Random|RandomBoolwithWeight (Variables|Default|GetForestDensity))
        (ChildActorComponent|SetChildActorClass _returnvalue "/Game/Blueprints/BP_ForestTile.BP_ForestTile_C")
        (elif (Math|Random|RandomBoolwithWeight 0.2)
          (ChildActorComponent|SetChildActorClass _returnvalue "/Game/Blueprints/BP_FieldTile.BP_FieldTile_C")
          (else
            (ChildActorComponent|SetChildActorClass _returnvalue "/Game/Blueprints/BP_RockTile.BP_RockTile_C")))))
    (Utilities|FlowControl|FlipFlop
      (:A
        (Variables|Default|SetRowOffset (* (Variables|Default|GetTileRadius) -1.0)))
      (:B
        (Variables|Default|SetRowOffset 0.0)))))