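; BP_SplineWall is an actor that builds a wall from repeated spline mesh segments along its Spline.
; The construction script divides the spline length by MeshLength and adds one attached spline mesh component per whole segment, leaving any shorter remainder uncovered.
; Each segment takes its local-space endpoints and tangents from the spline, with tangent size clamped to at most MeshLength.
; The event graph is unused.
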(event EventBeginPlay)

(event Collision|EventActorBeginOverlap
  (params (OtherActor :type Actor%20Object%20Reference)))

(event EventTick
  (params (DeltaSeconds :type Float%20%28single-precision%29)))

(fn ConstructionScript
  (bind _spline (Variables|Default|GetSpline))
  (bind _meshlength (Variables|Default|GetMeshLength))
  (bind _spline_2 (Variables|Default|GetSpline))
  (bind _spline_3 (Variables|Default|GetSpline))
  (bind _returnvalue (Spline|GetSplineLength _spline))
  (bind _returnvalue_2 (/ _returnvalue _meshlength))
  (bind _returnvalue_3 (Math|Float|Truncate _returnvalue_2))
  ;[1 1 1] Calculate number of meshes
  (if (> _returnvalue_3 0)
    (for _index (range 0 (- _returnvalue_3 1))
      ;[1 1 1] Add spline mesh component
      (bind _returnvalue_4 (AddComponent|AddSplineMeshComponent false))
      (SplineMesh|SetStartandEnd _returnvalue_4 (Spline|GetLocationatDistanceAlongSpline _spline_3 (* _index (Variables|Default|GetMeshLength)) "Local") (Math|Vector|ClampVectorSize (Spline|GetTangentatDistanceAlongSpline _spline_3 (* _index (Variables|Default|GetMeshLength)) "Local") 1.0 (Variables|Default|GetMeshLength)) (Spline|GetLocationatDistanceAlongSpline _spline_2 (* (+ _index 1) (Variables|Default|GetMeshLength)) "Local") (Math|Vector|ClampVectorSize (Spline|GetTangentatDistanceAlongSpline _spline_2 (* (+ _index 1) (Variables|Default|GetMeshLength)) "Local") 1.0 (Variables|Default|GetMeshLength)) true :!class /Script/Engine.SplineMeshComponent)
      (Transformation|AttachComponentToComponent _returnvalue_4 (Variables|Default|GetSpline) "None" "KeepRelative" "KeepRelative" "KeepRelative" true))))